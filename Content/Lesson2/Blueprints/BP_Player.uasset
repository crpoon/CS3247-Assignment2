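; BP_Player is a VR player Blueprint that fires bullets and reacts to being hit.
; Pressing Space Bar calls SpawnBullets, which spawns a BP_Bullet just in front of the VR camera, facing its forward vector.
; Any overlap on the Sphere component prints a hit message and plays an explosion sound at the player's location.
; A looping auto-fire timer is present but unconnected, so it never runs.
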(event OnComponentBeginOverlap(Sphere)
  (params (OtherActor :type Actor%20Object%20Reference) (OtherComp :type Primitive%20Component%20Object%20Reference) (OtherBodyIndex :type Integer) (bFromSweep :type Boolean) (SweepResult :type Hit%20Result%20Structure%20%28by%20ref%29))
  ;[1 1 1] Collision Detection
  (Development|PrintString "The player has been hit!")
  (Audio|PlaySoundatLocation "/Game/MobileStarterContent/Audio/Explosion01.Explosion01" (Transformation|GetActorLocation)))

(event EventBeginPlay)

(event EventActorBeginOverlap
  (params (OtherActor :type Actor%20Object%20Reference)))

(event EventTick
  (params (DeltaSeconds :type Float%20%28single-precision%29)))

(event EventBeginPlay
  ;[1 1 1] Spawn Bullets
)

(event Input|KeyboardEvents|SpaceBar
  (params (Key :type Key%20Structure :default "AnyKey"))
  ;[1 1 1] Spawn Bullets
  (:Pressed
    (CallFunction|SpawnBullets)))

(fn ConstructionScript)

(fn SpawnBullets
  (bind (_location _forward_vector) (CallFunction|GetPlayerVRCameraProperties))
  (Game|SpawnActorfromClass "/Game/Lesson2/Blueprints/BP_Bullet.BP_Bullet_C" (Math|Transform|MakeTransform (+ _location (* _forward_vector 6e+01)) (Math|Conversions|RotationFromXVector _forward_vector)) "Undefined" 0 0)
  (return))