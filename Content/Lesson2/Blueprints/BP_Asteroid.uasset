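; BP_Asteroid is an asteroid actor that spins and homes in on the player, exploding and awarding a point on overlap.
; BeginPlay draws a debug "Hello World" label and picks a random spin.
; Tick sweeps it toward the player pawn at a multiple of BP_HUD's speed, without delta-time scaling.
; Any mesh overlap spawns explosion effects, destroys the actor and increments the score stored on BP_HUD.
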(event OnComponentBeginOverlap(StaticMesh)
  (params (OtherActor :type Actor%20Object%20Reference) (OtherComp :type Primitive%20Component%20Object%20Reference) (OtherBodyIndex :type Integer) (bFromSweep :type Boolean) (SweepResult :type Hit%20Result%20Structure%20%28by%20ref%29))
  (bind _returnvalue (Transformation|GetActorLocation))
  ;[1 1 1] Destroy on Collision
  (Effects|SpawnEmitteratLocation "/Game/MobileStarterContent/Particles/P_Explosion.P_Explosion" _returnvalue)
  (Audio|PlaySoundatLocation "/Game/EpicsMobileStarterContent/Audio/Explosion02.Explosion02" _returnvalue)
  (Actor|DestroyActor)
  ;[1 1 1] Add Score
  (bind _asbp_hud (CallFunction|GetHUD))
  (bind _asbp_hud_2 (CallFunction|GetHUD))
  (Variables|/Game/Lesson2/Blueprints/BP_HUD.BP_HUD_C|SetHUD%20Score _asbp_hud_2 (+ (Variables|/Game/Lesson2/Blueprints/BP_HUD.BP_HUD_C|GetHUD%20Score _asbp_hud) 1)))

(event EventBeginPlay
  ;[1 1 1] Hello World String
  (CallFunction|DrawVRDebugString "Hello  World" (+ (Transformation|GetActorLocation) "0, 0,200.000000") 5.0 "(R=0.000000,G=0.906580,B=1.000000,A=1.000000)")
  ;[1 1 1] Set Rotation Speed
  (Variables|Default|SetRotationSpeed (Math|Rotator|MakeRotator (Math|Random|RandomFloatinRange 1.0 15.0) (Math|Random|RandomFloatinRange 1.0 15.0) (Math|Random|RandomFloatinRange 1.0 15.0))))

(event EventTick
  (params (DeltaSeconds :type Float%20%28single-precision%29))
  ;[1 1 1] Move Towards the Player @ 5x
  (bind _asbp_hud (CallFunction|GetHUD))
  (Transformation|AddActorWorldOffset (* (Class|KismetMathLibrary|GetDirectionVector (Transformation|GetActorLocation) (Transformation|GetActorLocation (Game|Player|GetPlayerPawn 0))) (* (Variables|/Game/Lesson2/Blueprints/BP_HUD.BP_HUD_C|GetHUD%20Speed _asbp_hud) 5)) true)
  ;[1 1 1] Rotate on tick
  (Transformation|AddWorldRotation (Variables|Default|GetStaticMesh) (Variables|Default|GetRotationSpeed) false false))

(fn ConstructionScript)

(fn GetHUD
  (bind _asbp_hud (Utilities|Casting|CastToBP_HUD (HUD|GetHUD (Game|GetPlayerController 0)))
    (:then
      _)
    (:CastFailed
      _))
  (return _asbp_hud))